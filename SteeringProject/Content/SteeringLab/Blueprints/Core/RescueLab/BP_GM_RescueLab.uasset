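; Game mode for the Rescue Lab level, coordinating rescuer characters toward victims.
; BeginPlay shows the rescuer widget, gathers hospitals and victims (printing warnings if none exist), then spawns rescuers at preset starting positions.
; Every tick, it sends the first victim's mesh location as a rescue mission to a randomly chosen rescuer, whose random index excludes the last one spawned.
; A Menu event returns to the main menu.
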(event EventBeginPlay
  (bind _returnvalue (UserInterface|CreateWidget "/Game/SteeringLab/Widgets/WB_Rescuer_Main.WB_Rescuer_Main_C"))
  (bind _output_get (Variables|Components|SetWidget%20Rescuer _returnvalue))
  (UserInterface|Viewport|AddtoViewport _output_get 0)
  (Setup|SetupLevel))

(event EventMenu
  (Game|OpenLevel(byObjectReference) "/Game/SteeringLab/Maps/MAP_MainMenu.MAP_MainMenu"))

(event EventTick
  (params (DeltaSeconds :type Float%20%28single-precision%29))
  (if (not (Utilities|Array|IsEmpty (Variables|Rescuers|GetTargets)))
    (Class|BPIRescuerControl|RescueMission(Message) (Mission|RescuerChooser) (Transformation|GetWorldLocation (Variables|/Script/Engine.Character|GetMesh (Utilities|Array|Get(acopy) (Variables|Rescuers|GetTargets)))))))

(fn ConstructionScript)

(fn SetupLevel
  (Setup|GetAllActors)
  (Setup|SpawnRescuers))

(fn SpawnRescuers
  (for _array_element (Variables|Rescuers|GetStartingPositions)
    (bind _returnvalue (Game|SpawnActorfromClass "/Game/SteeringLab/Blueprints/Characters/NonPlayable/BP_RescuerCharacter.BP_RescuerCharacter_C" (Math|Transform|MakeTransform _array_element "0.000000,-180.000000,0.000000" "1.000000,1.000000,1.000000") "Undefined" "MultiplyWithRoot" 0 0))
    (Utilities|Array|Add (Variables|Rescuers|GetRescuers) _returnvalue)))

(fn GetAllActors
  (Utilities|FlowControl|Sequence
    (:then_0
      (bind _outactors (Actor|GetAllActorsOfClass "/Game/SteeringLab/Blueprints/Actors/A_Hospital.A_Hospital_C"))
      (Variables|Hospital|SetHospitals _outactors)
      (bind _outactors_2 (Actor|GetAllActorsOfClass "/Game/SteeringLab/Blueprints/Characters/NonPlayable/BP_VictimCharacter.BP_VictimCharacter_C"))
      (Variables|Rescuers|SetTargets _outactors_2))
    (:then_1
      (if (Utilities|Array|IsEmpty (Variables|Hospital|GetHospitals))
        (Development|PrintString "No hospital found" true true "(R=1.000000,G=0.000000,B=0.000000,A=1.000000)" 12.0)))
    (:then_2
      (if (Utilities|Array|IsEmpty (Variables|Rescuers|GetTargets))
        (Development|PrintString "No target found" true true "(R=1.000000,G=0.000000,B=0.000000,A=1.000000)" 12.0)))))

(fn RescuerChooser
  (return (Utilities|Array|Get(acopy) (Variables|Rescuers|GetRescuers) (Math|Random|RandomInteger (- (Utilities|Array|Length (Variables|Rescuers|GetRescuers)) 1)))))