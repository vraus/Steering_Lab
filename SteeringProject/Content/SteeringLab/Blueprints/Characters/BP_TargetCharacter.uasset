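; BP_TargetCharacter is the AI-moved target character that reacts to the player's current steering behaviour.
; On BeginPlay it registers with the top-down controller and binds to the player character's behaviour-changed event.
; Seek, Flee and Arrival stop it, Pursuit makes it wander to random nearby points, and Evade makes it chase the player.
; Both movement modes re-issue AIMoveTo on success or failure while ShouldMove is set.
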(event Custom|onBehaviorChanged
  (params (Behaviour :type EBehaviours%20Enum :default "Undefined"))
  (switch Utilities|FlowControl|Switch|SwitchonEBehaviours Behaviour
    (:Seek
      (Variables|SteeringBehavior|SetbShouldMove false :!label _label)
      (Components|Movement|StopMovementImmediately (Variables|Character|GetCharacterMovement)))
    (:Flee
      (goto _label))
    (:Pursuit
      (Variables|SteeringBehavior|SetbShouldMove true)
      (CallFunction|MovetoRandomLocation))
    (:Evade
      (Variables|SteeringBehavior|SetbShouldMove true)
      (CallFunction|ChasePlayer))
    (:Arrival
      (goto _label))))

(event Custom|MoveToRandomLocation
  (if (Variables|SteeringBehavior|GetbShouldMove)
    (AI|AIMoveTo self (Variables|SteeringBehavior|GetAIMoveToLocation) 0 5.0 false
      (:then
        (bind _new_location (CallFunction|PickNewRandomLocation))
        (Variables|SteeringBehavior|SetAIMoveToLocation _new_location))
      (:OnSuccess
        (CallFunction|MovetoRandomLocation :!label _label))
      (:OnFail
        (goto _label)))))

(event Custom|ChasePlayer
  (if (Variables|SteeringBehavior|GetbShouldMove)
    (AI|AIMoveTo self "0, 0, 0" (Game|Player|GetPlayerPawn 0) 5.0 false
      (:OnSuccess
        _)
      (:OnFail
        _))
    (CallFunction|ChasePlayer)))

(event EventBeginPlay
  (bind _new_location (CallFunction|PickNewRandomLocation))
  (Variables|SteeringBehavior|SetAIMoveToLocation _new_location)
  (Class|SteeringPlayerController|SetTargetCharacter (.AsBP%20Top%20Down%20Controller (Utilities|Casting|CastToBP_TopDownController (Game|GetPlayerController 0))) self)
  (EventDispatchers|BindEventtoEDonBehaviourChanged (.AsBP%20Top%20Down%20Character (Utilities|Casting|CastToBP_TopDownCharacter (Game|Player|GetPlayerPawn 0))) (delegate Custom|onBehaviorChanged)))

(fn ConstructionScript)

(fn PickNewRandomLocation
  (return (+ (Transformation|GetActorLocation) (* (Class|KismetMathLibrary|VectorNormal2D (Math|Random|RandomUnitVector) 0.0001) (* (Math|Random|RandomFloat) 1.5e+03)))))