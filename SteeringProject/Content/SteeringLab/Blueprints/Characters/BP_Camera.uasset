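; Free-fly camera for SteeringLab, driven by Enhanced Input for planar movement, vertical movement and mouse look.
; Movement applies local actor offsets without sweep; yaw rotates the actor while pitch rotates only the camera, keeping movement level.
; Look input is ignored while the mouse cursor is visible.
; A FlipFlop on the slow-mode input toggles between reduced move and rotation sensitivities and hard-coded defaults.
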(event Input|EnhancedActionEvents|EnhancedInputActionIA_Move
  (params (ActionValue :type Vector%202D%20Structure) (ElapsedSeconds :type Float%20%28double-precision%29) (TriggeredSeconds :type Float%20%28double-precision%29) (InputAction :type Input%20Action%20Object%20Reference :default "/Game/SteeringLab/Blueprints/Input/Actions/IA_Move.IA_Move"))
  (bind _movesensibility (Variables|Input|GetMoveSensibility))
  (Transformation|AddActorLocalOffset (Math|Vector|MakeVector (* (.x ActionValue) _movesensibility) (* (.y ActionValue) _movesensibility) 0.0) false false))

(event Input|EnhancedActionEvents|EnhancedInputActionIA_Look
  (params (ActionValue :type Vector%202D%20Structure) (ElapsedSeconds :type Float%20%28double-precision%29) (TriggeredSeconds :type Float%20%28double-precision%29) (InputAction :type Input%20Action%20Object%20Reference :default "/Game/SteeringLab/Blueprints/Input/Actions/IA_Look.IA_Look"))
  (if (not (Variables|/Script/Engine.PlayerController|GetbShowMouseCursor (Game|GetPlayerController 0)))
    (Transformation|AddActorLocalRotation (Math|Rotator|MakeRotator 0.0 0.0 (* (.x ActionValue) (Variables|Input|GetRotationSensibility))) false false)
    (Transformation|AddLocalRotation (Variables|Default|GetCamera) (Math|Rotator|MakeRotator 0.0 (* (.y ActionValue) (Variables|Input|GetRotationSensibility)) 0.0) false false)))

(event Input|EnhancedActionEvents|EnhancedInputActionIA_UpDown
  (params (ActionValue :type Float%20%28double-precision%29) (ElapsedSeconds :type Float%20%28double-precision%29) (TriggeredSeconds :type Float%20%28double-precision%29) (InputAction :type Input%20Action%20Object%20Reference :default "/Game/SteeringLab/Blueprints/Input/Actions/IA_UpDown.IA_UpDown"))
  (Transformation|AddActorLocalOffset (Math|Vector|MakeVector 0.0 0.0 (* ActionValue (Variables|Input|GetMoveSensibility))) false false))

(event Input|EnhancedActionEvents|EnhancedInputActionIA_SlowMode
  (params (ActionValue :type Boolean) (ElapsedSeconds :type Float%20%28double-precision%29) (TriggeredSeconds :type Float%20%28double-precision%29) (InputAction :type Input%20Action%20Object%20Reference :default "/Game/SteeringLab/Blueprints/Input/Actions/IA_SlowMode.IA_SlowMode"))
  (:Started
    (Utilities|FlowControl|FlipFlop
      (:A
        (Input|SlowMode))
      (:B
        (Input|SetSensibilitytoDefault)))))

(fn ConstructionScript)

(fn SetSensibilitytoDefault
  (Variables|Input|SetRotationSensibility 5.0)
  (Variables|Input|SetMoveSensibility 2e+01))

(fn SlowMode
  (Variables|Input|SetMoveSensibility (/ (Variables|Input|GetMoveSensibility) 4.0))
  (Variables|Input|SetRotationSensibility (/ (Variables|Input|GetRotationSensibility) 2.0)))